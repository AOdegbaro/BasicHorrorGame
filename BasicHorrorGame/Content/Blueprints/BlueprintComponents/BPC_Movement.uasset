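; Movement component that handles sprinting with stamina and crouching for the player character by changing max walk speed.
; Sprint requires stamina and movement, then drains stamina on a looping timer and stops when empty or stationary.
; Stopping sprint starts timed stamina regeneration after a retriggerable delay.
; Crouching cancels the sprint drain and calls L1_PlayerCharacter to shorten or lengthen its capsule.
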(event `StartSprint`
  ;[1 0.8822 0.1622] Have Player start Sprinting
  ;;[1 0.1872 0.2071] Check to if player is crouching first
  (if (`self.IsCrouching`)
    (`self.StopCrouch`))
  (if (and (> (`self.CurrentStamina`) (`self.MinStamina`)) (> (`KismetMathLibrary.VSize` (`Actor.GetVelocity` (`self.Player Ref`))) 10.0))
    ;;[1 0.1872 0.2071] Stop Regenerating Stamina
    (`KismetSystemLibrary.K2_ClearTimer` null "RegenerateStamina")
    (`self.SetPlayerMaxWalkSpeed` (`self.SprintSpeed`))
    (`KismetSystemLibrary.K2_SetTimer` null "SprintTimer" 0.1 true)))

(event `StartCrouch`
  ;[1 0.8822 0.1622] Starting Player Crouch Action
  (`KismetSystemLibrary.K2_ClearTimer` null "SprintTimer")
  (`self.SetPlayerMaxWalkSpeed` (`self.CrouchSpeed`))
  (`/Game/GameBP/Level1/L1_PlayerCharacter.ShortenPlayerCapsule` (cast `/Game/GameBP/Level1/L1_PlayerCharacter` (`self.Player Ref`) :!pure true))
  (set `self.IsCrouching` true))

(event `StopCrouch`
  ;[1 0.8822 0.1622] Stop player from crouching
  (`self.SetPlayerMaxWalkSpeed` (`self.WalkSpeed`))
  (`/Game/GameBP/Level1/L1_PlayerCharacter.LengthenPlayerCapsule` (cast `/Game/GameBP/Level1/L1_PlayerCharacter` (`self.Player Ref`) :!pure true))
  (set `self.IsCrouching` false))

(event `SprintTimer`
  ;[1 0.8822 0.1622] Decrease Stamina
  (if (> (`KismetMathLibrary.VSize` (`Actor.GetVelocity` (`self.Player Ref`))) 10.0)
    (bind _output_get (set `self.CurrentStamina` (`KismetMathLibrary.FClamp` (- (`self.CurrentStamina`) 1.0) (`self.MinStamina`) (`self.MaxStamina`))))
    ;;[0.217 1 0.4691] Debug
    (`KismetSystemLibrary.PrintString` (`KismetStringLibrary.Conv_DoubleToString` _output_get))
    (if (<= (`self.CurrentStamina`) (`self.MinStamina`))
      (`self.StopSprint`))
    (else
      ;;[1 0.1872 0.2071] If player has stopped moving whiling sprinting stop sprint and stop decreasing stamina
      (`self.StopSprint`))))

(event `StopSprint`
  ;[1 0.8822 0.1622] Stop Player from Sprinting
  ;;[1 0.1872 0.2071] Check to see if player is crouching
  (if (not (`self.IsCrouching`))
    (`KismetSystemLibrary.K2_ClearTimer` null "SprintTimer")
    (`self.SetPlayerMaxWalkSpeed` (`self.WalkSpeed`))
    ;;[1 0.1872 0.2071] Check to see if player stopped sprinting to regenerate stamina
    (`KismetSystemLibrary.RetriggerableDelay` 5.0)
    (if (not (`KismetSystemLibrary.K2_IsTimerActive` null "SprintTimer"))
      (`KismetSystemLibrary.K2_SetTimer` null "RegenerateStamina" 0.03 true))))

(event `RegenerateStamina`
  ;[1 0.8822 0.1622] Regenerate Player Stamina
  (bind _output_get (set `self.CurrentStamina` (`KismetMathLibrary.FClamp` (+ (`self.CurrentStamina`) 1.0) (`self.MinStamina`) (`self.MaxStamina`))))
  ;;[0.217 1 0.4691] Debug
  (`KismetSystemLibrary.PrintString` (`KismetStringLibrary.Conv_DoubleToString` _output_get))
  (if (>= (`self.CurrentStamina`) (`self.MaxStamina`))
    (`KismetSystemLibrary.K2_ClearTimer` null "RegenerateStamina")))

(fn `Initalize`
  (params (Character :type "Character Object Reference"))
  (set `self.Player Ref` Character)
  (set `CharacterMovementComponent.MaxWalkSpeed` (`self.WalkSpeed`) (`Character.CharacterMovement` (`self.Player Ref`))))

(fn `SetPlayerMaxWalkSpeed`
  (params (`Max Walk Speed` :type "Float (double-precision)"))
  (set `CharacterMovementComponent.MaxWalkSpeed` `Max Walk Speed` (`Character.CharacterMovement` (`self.Player Ref`))))